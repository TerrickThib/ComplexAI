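; Enemy AI Blueprint that spawns short-range weapons while the player character is nearby.
; The SpawnShortWeapon event starts a looping timer that runs SpawnShortRange each second, spawning a WeaponShortRange at the ArrowNew transform if the player is within range.
; The PickUpWeapon event pauses that timer.
; Tick prints the enemy's distance to the player on screen.
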(event `self.ReceiveTick`
  (params (DeltaSeconds :type "Float (single-precision)"))
  ;[1 1 1] Finds the distance between the EnemyAI and the player Character and displays it on screen.
  (`KismetSystemLibrary.PrintString` (`KismetStringLibrary.Conv_DoubleToString` (`KismetMathLibrary.VSize` (- (`self.K2_GetActorLocation` self) (`self.K2_GetActorLocation` (`GameplayStatics.GetPlayerCharacter` 0)))))))

(event `SpawnShortWeapon`
  ;[1 1 1] Creates custom event that calls the function SpawnShortRange every second.
  (`KismetSystemLibrary.K2_SetTimer` null "SpawnShortRange" 1.0 true))

(event `PickUpWeapon`
  ;[1 1 1] Created custom event pick up weapon. When called stops Function SpawnShortRange
  (`KismetSystemLibrary.K2_PauseTimer` null "SpawnShortRange"))

(fn `SpawnShortRange`
  ;[1 1 1] Gets the distance from charater to Enemy. If distance is within 1000 units then spawn short range meets the condition and can go into true otherwise it is false
  (if (< (`self.GetDistanceTo` (`GameplayStatics.GetPlayerCharacter` 0)) 1000.0)
    (`|SpawnActorFromClass` "/Game/Enemy/WeaponShortRange.WeaponShortRange_C" (`SceneComponent.K2_GetComponentToWorld` (`self.ArrowNew`)) "Undefined" "OverrideRootScale" null null)))

(fn `UserConstructionScript`)